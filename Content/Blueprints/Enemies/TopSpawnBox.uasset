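; TopSpawnBox is an enemy spawner that periodically spawns actors, noted as the "down enemy", at random points inside its TopBox volume.
; A Delay on Tick acts as a repeating timer.
; After each wait it casts the player pawn to TopDownCharacter and spawns only if TimeCheck is set and HitCheck and PausedCheck are clear.
; Spawn collision handling adjusts the location or skips the spawn when blocked.
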(event EventTick
  (params (DeltaSeconds :type Float%20%28single-precision%29))
  (bind _topbox (Variables|Default|GetTopBox))
  ;[1 0 0.06667] Random spawns for down enemy
  (Utilities|FlowControl|Delay (Math|Conversions|ToFloat(Integer) 7))
  (bind _astop_down_character (Utilities|Casting|CastToTopDownCharacter (Game|Player|GetPlayerPawn 0)))
  (if (Variables|/Game/Blueprints/TopDownCharacter.TopDownCharacter_C|GetTimeCheck _astop_down_character)
    (if (not (Variables|/Game/Blueprints/TopDownCharacter.TopDownCharacter_C|GetHitCheck _astop_down_character))
      (if (not (Variables|/Game/Blueprints/TopDownCharacter.TopDownCharacter_C|GetPausedCheck _astop_down_character))
        (Game|SpawnActorfromClass "/Game/Blueprints/Enemies/DownEnemy.DownEnemy_C" (Math|Conversions|ToTransform(Vector) (Math|Random|RandomPointinBoundingBox (Transformation|GetWorldLocation _topbox) (Components|Box|GetScaledBoxExtent _topbox))) "AdjustIfPossibleButDontSpawnIfColliding" 0 0)))))

(fn ConstructionScript)