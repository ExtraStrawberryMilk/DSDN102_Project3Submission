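; DownEnemy is an enemy that moves vertically by its Speed every tick and destroys itself after 15 seconds.
; Each tick it checks the player's Score, lowering Speed by a fixed step whenever a rising threshold is reached.
; Capsule hits flag the player's HitCheck or destroy blocks.
; Hitting sides, fragments or Across and Diag enemies briefly disables the movement sweep so it passes through.
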(event OnComponentHit(CapsuleComponent)
  (params (HitComponent :type Primitive%20Component%20Object%20Reference) (OtherActor :type Actor%20Object%20Reference) (OtherComp :type Primitive%20Component%20Object%20Reference) (NormalImpulse :type Vector :default "0, 0, 0") (Hit :type Hit%20Result%20Structure%20%28by%20ref%29))
  ;[1 0 0.06667] All compents hits for enemy
  (Utilities|Casting|CastToSides OtherActor
    (:then
      (Variables|Default|SetSideHit false :!label _label)
      (Utilities|FlowControl|Delay 0.5)
      (Variables|Default|SetSideHit true))
    (:CastFailed
      (Utilities|Casting|CastToSqaureFragment OtherActor
        (:then
          (goto _label))
        (:CastFailed
          (bind _astop_down_character (Utilities|Casting|CastToTopDownCharacter OtherActor)
            (:then
              (Variables|/Game/Blueprints/TopDownCharacter.TopDownCharacter_C|SetHitCheck _astop_down_character true))
            (:CastFailed
              (bind _asblock_1 (Utilities|Casting|CastToBlock1 OtherActor)
                (:then
                  (Default|Destroy _asblock_1))
                (:CastFailed
                  (bind _asblock_2 (Utilities|Casting|CastToBlock2 OtherActor)
                    (:then
                      (Default|Destroy _asblock_2))
                    (:CastFailed
                      (bind _asblock_3 (Utilities|Casting|CastToBlock3 OtherActor)
                        (:then
                          (Default|Destroy _asblock_3))
                        (:CastFailed
                          (Utilities|Casting|CastToAcrossEnemy OtherActor
                            (:then
                              (goto _label))
                            (:CastFailed
                              (Utilities|Casting|CastToDiagEnemy OtherActor)
                              (goto _label))))))))))))))))

(event Custom|setSpeed
  ;[1 0 0.06663] Variation Speed Set
  (bind _astop_down_character (Utilities|Casting|CastToTopDownCharacter (Game|Player|GetPlayerPawn 0)))
  (if (>= (Variables|/Game/Blueprints/TopDownCharacter.TopDownCharacter_C|GetScore _astop_down_character) (Variables|Default|GetscoreCheck))
    (Variables|Default|SetscoreCheck (+ (Variables|Default|GetscoreCheck) 5.0))
    (Variables|Default|Setspeed (+ (Variables|Default|Getspeed) -0.5))))

(event EventTick
  (params (DeltaSeconds :type Float%20%28single-precision%29))
  ;[1 0 0.06663] Moves enemy down every tick
  (CallFunction|SetSpeed)
  (if true
    (Transformation|SetActorTransform (Math|Transform|MakeTransform (+ (Transformation|GetActorLocation) (Math|Vector|MakeVector 0.0 0.0 (Variables|Default|Getspeed))) "0, 0, 0" "1.000000,1.000000,1.000000") (Variables|Default|GetSideHit))
    (Utilities|FlowControl|Delay 15.0)
    (Actor|DestroyActor)))

(fn ConstructionScript)