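; DiagEnemy is an enemy that moves diagonally along the Y-Z plane at a fixed X, destroying itself after a 15-second delay.
; Tick steps its transform by a fixed, frame-rate-dependent offset, using SideHit as the sweep flag.
; Capsule hits flag HitCheck on TopDownCharacter and destroy Block1-3 actors.
; Hits on sides, square fragments, AcrossEnemy or DownEnemy briefly disable sweeping so it passes through.
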(event OnComponentHit(CapsuleComponent)
  (params (HitComponent :type Primitive%20Component%20Object%20Reference) (OtherActor :type Actor%20Object%20Reference) (OtherComp :type Primitive%20Component%20Object%20Reference) (NormalImpulse :type Vector :default "0, 0, 0") (Hit :type Hit%20Result%20Structure%20%28by%20ref%29))
  ;[1 0 0.06667] All compents hit for the enemy
  (Utilities|Casting|CastToSides OtherActor
    (:then
      (Variables|Default|SetSideHit false :!label _label)
      (Utilities|FlowControl|Delay 0.8)
      (Variables|Default|SetSideHit true))
    (:CastFailed
      (Utilities|Casting|CastToSqaureFragment OtherActor
        (:then
          (goto _label))
        (:CastFailed
          (bind _astop_down_character (Utilities|Casting|CastToTopDownCharacter OtherActor)
            (:then
              (Variables|/Game/Blueprints/TopDownCharacter.TopDownCharacter_C|SetHitCheck _astop_down_character true))
            (:CastFailed
              (bind _asblock_1 (Utilities|Casting|CastToBlock1 OtherActor)
                (:then
                  (Default|Destroy _asblock_1))
                (:CastFailed
                  (bind _asblock_2 (Utilities|Casting|CastToBlock2 OtherActor)
                    (:then
                      (Default|Destroy _asblock_2))
                    (:CastFailed
                      (bind _asblock_3 (Utilities|Casting|CastToBlock3 OtherActor)
                        (:then
                          (Default|Destroy _asblock_3))
                        (:CastFailed
                          (Utilities|Casting|CastToAcrossEnemy OtherActor
                            (:then
                              (goto _label))
                            (:CastFailed
                              (Utilities|Casting|CastToDownEnemy OtherActor)
                              (goto _label))))))))))))))))

(event EventTick
  (params (DeltaSeconds :type Float%20%28single-precision%29))
  (bind _returnvalue (Transformation|GetActorLocation))
  ;[1 0 0.06667] Moves enemy diagonal every tick
  (Variables|Default|SetstartVector (Math|Vector|MakeVector 6.6e+02 (.y _returnvalue) (.z _returnvalue)))
  (Transformation|SetActorTransform (Math|Transform|MakeTransform (- (Variables|Default|GetstartVector) "0.000000,-2.000000,1.051000") "0.000000,90.000000,0.000000" "2.000000,1.000000,1.000000") (Variables|Default|GetSideHit))
  (Utilities|FlowControl|Delay 15.0)
  (Actor|DestroyActor))

(fn ConstructionScript)