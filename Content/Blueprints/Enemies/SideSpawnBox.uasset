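; SideSpawnBox is a spawner that places AcrossEnemy actors at random points inside its SideBox volume.
; Tick feeds a 10-second Delay, making it a repeating timer that then checks the player's TopDownCharacter.
; A spawn happens only while TimeCheck is true and HitCheck and PausedCheck are false, adjusting position to avoid collisions or skipping if none fits.
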(event EventTick
  (params (DeltaSeconds :type Float%20%28single-precision%29))
  (bind _sidebox (Variables|Default|GetSideBox))
  ;[1 0 0.06667] Random spawns for across enemy
  (Utilities|FlowControl|Delay (Math|Conversions|ToFloat(Integer) 10))
  (bind _astop_down_character (Utilities|Casting|CastToTopDownCharacter (Game|Player|GetPlayerPawn 0)))
  (if (Variables|/Game/Blueprints/TopDownCharacter.TopDownCharacter_C|GetTimeCheck _astop_down_character)
    (if (not (Variables|/Game/Blueprints/TopDownCharacter.TopDownCharacter_C|GetHitCheck _astop_down_character))
      (if (not (Variables|/Game/Blueprints/TopDownCharacter.TopDownCharacter_C|GetPausedCheck _astop_down_character))
        (Game|SpawnActorfromClass "/Game/Blueprints/Enemies/AcrossEnemy.AcrossEnemy_C" (Math|Conversions|ToTransform(Vector) (Math|Random|RandomPointinBoundingBox (Transformation|GetWorldLocation _sidebox) (Components|Box|GetScaledBoxExtent _sidebox))) "AdjustIfPossibleButDontSpawnIfColliding" 0 0)))))

(fn ConstructionScript)