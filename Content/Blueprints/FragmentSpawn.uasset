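; FragmentSpawn is a spawner that places SqaureFragment actors at random points inside its Box volume.
; BeginPlay spawns the first fragment, adjusting position if needed but always spawning.
; Tick polls the player TopDownCharacter's Collected flag and, when set, spawns a replacement that must find a collision-free spot.
; A failed spawn retries in an uncapped loop within the same frame; success clears the flag.
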(event EventBeginPlay
  (bind _box (Variables|Default|GetBox))
  ;[1 0.8627 0.2118] Iniital spawn of the fragment
  (Game|SpawnActorfromClass "/Game/Blueprints/SqaureFragment.SqaureFragment_C" (Math|Conversions|ToTransform(Vector) (Math|Random|RandomPointinBoundingBox (Transformation|GetWorldLocation _box) (Components|Box|GetScaledBoxExtent _box))) "AdjustIfPossibleButAlwaysSpawn" 0 0))

(event EventTick
  (params (DeltaSeconds :type Float%20%28single-precision%29))
  (bind _box (Variables|Default|GetBox))
  ;[1 0.8627 0.2118] Randomly spawns fragments
  (bind _astop_down_character (Utilities|Casting|CastToTopDownCharacter (Game|Player|GetPlayerPawn 0)))
  (if (Variables|/Game/Blueprints/TopDownCharacter.TopDownCharacter_C|GetCollected _astop_down_character)
    (bind _returnvalue (Game|SpawnActorfromClass "/Game/Blueprints/SqaureFragment.SqaureFragment_C" (Math|Conversions|ToTransform(Vector) (Math|Random|RandomPointinBoundingBox (Transformation|GetWorldLocation _box) (Components|Box|GetScaledBoxExtent _box))) "AdjustIfPossibleButDontSpawnIfColliding" 0 0 :!label _label))
    (Utilities|IsValid _returnvalue
      (:Is%20Valid
        (Variables|/Game/Blueprints/TopDownCharacter.TopDownCharacter_C|SetCollected _astop_down_character false))
      (:Is%20Not%20Valid
        (goto _label)))))

(fn ConstructionScript)